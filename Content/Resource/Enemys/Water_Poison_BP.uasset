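; Poison water hazard that drains the third-person character's Health while they are inside its Box trigger.
; Begin and end overlap toggle a poison flag through two DoOnce nodes that re-arm each other, with splash effects and sounds on entry and exit.
; While the flag is set, Tick uses Delays to pace damage to player 0 and, when they move, walking splashes with FlipFlop-alternated water footstep sounds.
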(event OnComponentBeginOverlap(Box)
  (params (OverlappedComponent :type Primitive%20Component%20Object%20Reference) (OtherActor :type Actor%20Object%20Reference) (OtherComp :type Primitive%20Component%20Object%20Reference) (OtherBodyIndex :type Integer) (bFromSweep :type Boolean) (SweepResult :type Hit%20Result%20Structure%20%28by%20ref%29))
  (bind _asthird_person_character (Utilities|Casting|CastToThirdPersonCharacter OtherActor))
  (Utilities|FlowControl|DoOnce false
    (:Completed
      (Effects|SpawnEmitteratLocation "/Game/Resource/SFXs/Water_Splash.Water_Splash" (Transformation|GetActorLocation _asthird_person_character))
      (Audio|PlaySound2D "/Game/Resource/Sound/Out_Water.Out_Water" 1.0 1.0 0.0 0 0)
      (Variables|Default|SetPosion? true)
      (Utilities|FlowControl|DoOnce false) ; enters at Reset
    )))

(event OnComponentEndOverlap(Box)
  (params (OverlappedComponent :type Primitive%20Component%20Object%20Reference) (OtherActor :type Actor%20Object%20Reference) (OtherComp :type Primitive%20Component%20Object%20Reference) (OtherBodyIndex :type Integer))
  (bind _asthird_person_character (Utilities|Casting|CastToThirdPersonCharacter OtherActor))
  (Utilities|FlowControl|DoOnce false
    (:Completed
      (Effects|SpawnEmitteratLocation "/Game/Resource/SFXs/Water_Splash.Water_Splash" (Transformation|GetActorLocation _asthird_person_character))
      (Variables|Default|SetPosion? false)
      (Audio|PlaySound2D "/Game/Resource/Sound/Walk_Water2.Walk_Water2" 1.0 1.0 0.0 0 0)
      (Utilities|FlowControl|DoOnce false) ; enters at Reset
    )))

(event EventTick
  (params (DeltaSeconds :type Float%20%28single-precision%29))
  (bind _returnvalue (Game|GetPlayerCharacter 0))
  (bind _returnvalue_2 (Transformation|GetActorLocation _returnvalue))
  (if (Variables|Default|GetPosion?)
    (Utilities|FlowControl|Sequence
      (:then_0
        (Utilities|FlowControl|Delay 0.4)
        (bind _asthird_person_character (Utilities|Casting|CastToThirdPersonCharacter (Game|GetPlayerCharacter 0)))
        (Variables|/Game/ThirdPersonBP/Blueprints/ThirdPersonCharacter.ThirdPersonCharacter_C|SetHealth _asthird_person_character (- (Variables|/Game/ThirdPersonBP/Blueprints/ThirdPersonCharacter.ThirdPersonCharacter_C|GetHealth _asthird_person_character) 1.0)))
      (:then_1
        (if (!= (Math|Vector|VectorLength (Transformation|GetVelocity _returnvalue)) 0.0)
          (Utilities|FlowControl|Delay 0.3)
          (Effects|SpawnEmitteratLocation "/Game/Resource/SFXs/Water_Splash_Walk.Water_Splash_Walk" _returnvalue_2)
          (Utilities|FlowControl|FlipFlop
            (:A
              (Audio|SpawnSoundatLocation "/Game/Resource/Sound/Walk_Water.Walk_Water" _returnvalue_2 "0, 0, 0" 0.3 1.0 0.0 0 0))
            (:B
              (Audio|SpawnSoundatLocation "/Game/Resource/Sound/Walk_Water2.Walk_Water2" _returnvalue_2 "0, 0, 0" 0.3 1.0 0.0 0 0))))))))

(fn ConstructionScript)