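; Letter_BP is a letter actor in the collectibles folder that shows an on-screen hint when the player character is nearby.
; On overlap of its Sphere by a ThirdPersonCharacter, it finds all top-level Hint widgets, passes them its ItemTypes enum as a string and makes them visible.
; When the character leaves the Sphere, it hides those widgets.
; The Blueprint contains no pickup logic of its own.
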(event OnComponentBeginOverlap(Sphere)
  (params (OverlappedComponent :type Primitive%20Component%20Object%20Reference) (OtherActor :type Actor%20Object%20Reference) (OtherComp :type Primitive%20Component%20Object%20Reference) (OtherBodyIndex :type Integer) (bFromSweep :type Boolean) (SweepResult :type Hit%20Result%20Structure%20%28by%20ref%29))
  (Utilities|Casting|CastToThirdPersonCharacter OtherActor)
  (bind _foundwidgets (Widget|GetAllWidgetsOfClass "/Game/Resource/UMG/Hint.Hint_C" true))
  (for _array_element _foundwidgets
    (Variables|/Game/Resource/UMG/Hint.Hint_C|SetItem%20Types _array_element (Utilities|String|EnumtoString (Variables|Default|GetItem%20Types)))
    (Widget|SetVisibility _array_element "Visible")))

(event OnComponentEndOverlap(Sphere)
  (params (OverlappedComponent :type Primitive%20Component%20Object%20Reference) (OtherActor :type Actor%20Object%20Reference) (OtherComp :type Primitive%20Component%20Object%20Reference) (OtherBodyIndex :type Integer))
  (Utilities|Casting|CastToThirdPersonCharacter OtherActor)
  (bind _foundwidgets (Widget|GetAllWidgetsOfClass "/Game/Resource/UMG/Hint.Hint_C" true))
  (for _array_element _foundwidgets
    (Widget|SetVisibility _array_element "Hidden")))

(fn ConstructionScript)